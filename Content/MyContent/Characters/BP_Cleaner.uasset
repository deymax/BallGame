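; BP_Cleaner is a roaming AI pawn that BP_Ball can shade red and other cleaners can restore to blue.
; It starts moving to random reachable points on BeginPlay, picking a new one only after each successful move.
; On Hit, a ball turns an original-colored cleaner red, while contact with an original-colored cleaner turns a red one blue.
; Each color change updates the shaded cube count in MyGameInstance.
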(event Custom|Random%20Roam
  ;[1 1 1] Movement
  (AI|AIMoveTo self (.RandomLocation (AI|Navigation|GetRandomReachablePointinRadius (Transformation|GetActorLocation) 2.5e+03 0 0)) 0 5.0 false
    (:OnSuccess
      (CallFunction|RandomRoam))))

(event EventBeginPlay
  ;[1 1 1] Movement
  (CallFunction|RandomRoam))

(event Collision|EventHit
  (params (MyComp :type Primitive%20Component%20Object%20Reference) (Other :type Actor%20Object%20Reference) (OtherComp :type Primitive%20Component%20Object%20Reference) (bSelfMoved :type Boolean) (HitLocation :type Vector :default "0, 0, 0") (HitNormal :type Vector :default "0, 0, 0") (NormalImpulse :type Vector :default "0, 0, 0") (Hit :type Hit%20Result%20Structure%20%28by%20ref%29))
  ;[1 1 1] Collisions
  (Utilities|Casting|CastToBP_Ball Other
    (:then
      (if (Variables|Default|GetIsOriginalColor)
        (Rendering|Material|SetMaterial (Variables|Character|GetMesh) 0 "/Game/MyContent/MyMaterials/Red.Red")
        (Variables|Default|SetIsOriginalColor false)
        (bind _asmy_game_instance (Utilities|Casting|CastToMyGameInstance (Game|GetGameInstance)))
        (Default|ChangeShadedСubesCount _asmy_game_instance true)))
    (:CastFailed
      (bind _asbp_cleaner (Utilities|Casting|CastToBP_Cleaner Other))
      (bind _original (CallFunction|GetColor _asbp_cleaner))
      (if _original
        (if (not (Variables|Default|GetIsOriginalColor))
          (Rendering|Material|SetMaterial (Variables|Character|GetMesh) 0 "/Game/MyContent/MyMaterials/Blue.Blue")
          (Variables|Default|SetIsOriginalColor true)
          (bind _asmy_game_instance_2 (Utilities|Casting|CastToMyGameInstance (Game|GetGameInstance)))
          (Default|ChangeShadedСubesCount _asmy_game_instance_2 false))))))

(fn ConstructionScript)

(fn GetColor
  (return (Variables|Default|GetIsOriginalColor)))